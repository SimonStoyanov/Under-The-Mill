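; TextRenderingActor is a trigger-box actor that shows a question as 3D text and opens a dialog widget on overlap.
; Begin overlap toggles the text's visibility, enables input, adds BP_DialogWidget to the viewport and shows the mouse cursor.
; End overlap and the Leaving event share one exit path that resets text and UpdateArray, removes all widgets, hides the cursor, then toggles visibility after a short delay.
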(event `self.Box.OnComponentBeginOverlap`
  (params (OverlappedComponent :type "PrimitiveComponent Object Reference") (OtherActor :type "Actor Object Reference") (OtherComp :type "PrimitiveComponent Object Reference") (OtherBodyIndex :type Integer) (bFromSweep :type Boolean) (SweepResult :type "HitResult Structure (by ref)"))
  (bind _returnvalue (`GameplayStatics.GetPlayerController` 0))
  (`SceneComponent.ToggleVisibility` (`self.TextRender`) false)
  (`self.EnableInput` (`GameplayStatics.GetPlayerController` 0))
  (`TextRenderComponent.K2_SetText` (`self.TextRender`) (`self.Question`))
  (bind _returnvalue_2 (`|CreateWidget` "/Game/Blueprints/Actors/BP_DialogWidget.BP_DialogWidget_C" _returnvalue))
  (`UserWidget.AddToViewport` _returnvalue_2 0)
  (bind _asplayer_controller (cast `PlayerController` _returnvalue))
  (set `PlayerController.bShowMouseCursor` true _asplayer_controller))

(event `self.Box.OnComponentEndOverlap`
  (params (OverlappedComponent :type "PrimitiveComponent Object Reference") (OtherActor :type "Actor Object Reference") (OtherComp :type "PrimitiveComponent Object Reference") (OtherBodyIndex :type Integer))
  (`self.DisableInput` (`GameplayStatics.GetPlayerController` 0) :!label _label)
  (`TextRenderComponent.K2_SetText` (`self.TextRender`) (`self.Question_0`))
  (set `self.UpdateArray` 0)
  (`WidgetLayoutLibrary.RemoveAllWidgets`)
  (bind _asplayer_controller (cast `PlayerController` (`GameplayStatics.GetPlayerController` 0)))
  (set `PlayerController.bShowMouseCursor` false _asplayer_controller)
  (`KismetSystemLibrary.Delay` 0.75)
  (`SceneComponent.ToggleVisibility` (`self.TextRender`) false))

(event `Leaving`
  (goto _label))

(fn `UserConstructionScript`)